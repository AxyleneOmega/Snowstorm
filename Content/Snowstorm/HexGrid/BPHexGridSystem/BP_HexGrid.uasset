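; Hex tile grid actor that builds breakable tiles as instanced static meshes and registers itself with the game mode.
; ConstructTiles lays out a hexagon-style grid from size, spacing and mesh bounds, at construction or on full regeneration.
; When the hit tile changes, the previous one is permanently scaled to FallenTileHeight on all axes, with custom instance data updated.
; Helpers return the tile count and a random tile location.
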(event EventBeginPlay
  (Class|IGM|RegisterHexGridActor(Message) (Game|GetGameMode) self))

(event EventBreakTileonCollision
  (params (HitItem :type Integer) (PrevHitItem :type Integer))
  (CallFunction|UpdateInstanceData PrevHitItem (!= HitItem PrevHitItem)))

(event EventRegenerateTiles
  (params (RegenerateAll? :type Boolean) (IndicesToRegenerate :type Set%20of%20Integers))
  (if RegenerateAll?
    (CallFunction|ConstructTiles)))

(fn ConstructionScript
  (CallFunction|ConstructTiles))

(fn UpdateInstanceData
  (params (InstanceIndex :type Integer) (Passed :type Boolean))
  (bind _fallentileheight (Variables|Default|GetFallenTileHeight))
  (bind _scale (Variables|HexGrid|GetScale))
  (bind _instancedstaticmesh (Variables|Default|GetInstancedStaticMesh))
  (bind _returnvalue (Math|Float|SelectFloat _fallentileheight _scale Passed))
  (bind _outinstancetransform (Components|InstancedStaticMesh|GetInstanceTransform _instancedstaticmesh InstanceIndex false))
  (bind _returnvalue_2 (== (.z (.scale _outinstancetransform)) _fallentileheight))
  (bind _returnvalue_3 (Math|Float|SelectFloat _fallentileheight _returnvalue _returnvalue_2))
  (Components|InstancedStaticMesh|UpdateInstanceTransform _instancedstaticmesh InstanceIndex (Math|Transform|MakeTransform (Math|Vector|MakeVector (.x (.location _outinstancetransform)) (.y (.location _outinstancetransform)) (.z (.location _outinstancetransform))) (.rotation _outinstancetransform) (Math|Vector|MakeVector _returnvalue_3 _returnvalue_3 _returnvalue_3)) false false false)
  (Components|InstancedStaticMesh|SetCustomDataValue _instancedstaticmesh InstanceIndex 0 (Math|Float|SelectFloat 1.0 -1.0 Passed) true))

(fn ConstructTiles
  (bind _instancedstaticmesh (Variables|Default|GetInstancedStaticMesh))
  (bind _size (Variables|HexGrid|GetSize))
  (bind _mesh (Variables|HexGrid|GetMesh))
  (bind _returnvalue (/ _size 2))
  (Components|InstancedStaticMesh|ClearInstances _instancedstaticmesh)
  (Components|StaticMesh|SetStaticMesh _instancedstaticmesh _mesh)
  (Variables|HexGrid|SetRadius (* (.x (.max (StaticMesh|GetBoundingBox _mesh))) (Variables|HexGrid|GetScale)))
  (switch Utilities|FlowControl|Switch|SwitchonE_HexCoordinateType (Variables|HexGrid|GetCoordinateType)
    (:NewEnumerator1
      (for _index (range (* _returnvalue -1) _returnvalue)
        (for _index_2 (range (* (/ (- (Variables|HexGrid|GetSize) (Math|Integer|Absolute(Integer) _index)) 2) -1) (- (/ (- (Variables|HexGrid|GetSize) (Math|Integer|Absolute(Integer) _index)) 2) (not (Math|Conversions|ToBoolean(Integer) (Math|Integer|%(Integer) (- (Variables|HexGrid|GetSize) (Math|Integer|Absolute(Integer) _index)) 2)))))
          (Components|InstancedStaticMesh|AddInstance (Variables|Default|GetInstancedStaticMesh) (Math|Transform|MakeTransform (Math|Vector|MakeVector (+ (* _index_2 (Variables|HexGrid|GetRadius) 2.0) (* _index_2 (Variables|HexGrid|GetSpacing)) (Math|Float|SelectFloat (- (Variables|HexGrid|GetRadius) (* (Variables|HexGrid|GetSpacing) -0.5)) 0.0 (not (Math|Conversions|ToBoolean(Integer) (Math|Integer|%(Integer) (- (Variables|HexGrid|GetSize) (Math|Integer|Absolute(Integer) _index)) 2))))) (Utilities|YCoord _index) 0.0) "0, 0, 0" (Math|Conversions|ToVector(Float) (Variables|HexGrid|GetScale))) false))))))

(fn GetRandomTileLocation
  (bind _instancedstaticmesh (Variables|Default|GetInstancedStaticMesh))
  (bind _returnvalue (Components|InstancedStaticMesh|GetInstanceCount _instancedstaticmesh))
  (bind _returnvalue_2 (Math|Random|RandomIntegerinRange 0 _returnvalue))
  (return _returnvalue_2 (.location (.OutInstanceTransform (Components|InstancedStaticMesh|GetInstanceTransform _instancedstaticmesh _returnvalue_2 true)))))

(fn GetTotalTiles
  (return (Components|InstancedStaticMesh|GetInstanceCount (Variables|Default|GetInstancedStaticMesh))))