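; Snowstorm game mode that spawns zombie, kamikaze and kraken enemies on random tiles of a registered hex grid.
; ToggleEnemySpawning flip-flops a looping timer per enemy type, picking a random interval from that type's data when started.
; Each wave spawns a configured count with custom gravity scale: zombies and kamikazes above tiles, krakens below.
; Only zombies have the grid show a shadow on their tile.
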(event Custom|Zombies
  (for _index (range 0 (- (.noofenemies (Variables|Default|GetZombieData)) 1))
    (bind _bp_hexgrid (Variables|Default|GetBP_HexGrid)
      (:then
        (bind (_tileindex _tilelocation) (Class|IHexGrid|GetRandomTileLocation(Message) _bp_hexgrid))
        (bind _returnvalue (Game|SpawnActorfromClass "/Game/Snowstorm/Systems/Enemies/BP_Enemy01.BP_Enemy01_C" (Math|Transform|MakeTransform (Math|Vector|MakeVector (.x _tilelocation) (.y _tilelocation) (+ (.z _tilelocation) 1e+03)) "0, 0, 0" "1.000000,1.000000,1.000000") "Undefined" "MultiplyWithRoot" 0 0))
        (Utilities|IsValid _returnvalue
          (:Is%20Valid
            (Class|IHexGrid|ShowShadow(Message) _bp_hexgrid _tileindex _returnvalue)
            (Variables|/Script/Engine.CharacterMovementComponent|SetGravityScale (Variables|/Script/Engine.Character|GetCharacterMovement _returnvalue) (.gravscale (Variables|Default|GetZombieData))))
          (:Is%20Not%20Valid
            (Development|PrintString "wompo womp"))))
      (:else))))

(event Custom|Kraken
  (for _index (range 0 (- (.noofenemies (Variables|Default|GetKrakenData)) 1))
    (bind _bp_hexgrid (Variables|Default|GetBP_HexGrid)
      (:then
        (bind _tilelocation (Class|IHexGrid|GetRandomTileLocation(Message) _bp_hexgrid))
        (bind _returnvalue (Game|SpawnActorfromClass "/Game/Snowstorm/Systems/Enemies/BP_Enemy03.BP_Enemy03_C" (Math|Transform|MakeTransform (Math|Vector|MakeVector (.x _tilelocation) (.y _tilelocation) (+ (.z _tilelocation) -1e+03)) "0.000000,180.000000,0.000000" "3.000000,3.000000,5.000000") "Undefined" "MultiplyWithRoot" 0 0))
        (Utilities|IsValid _returnvalue
          (:Is%20Valid
            (Variables|/Script/Engine.CharacterMovementComponent|SetGravityScale (Variables|/Script/Engine.Character|GetCharacterMovement _returnvalue) (.gravscale (Variables|Default|GetKrakenData))))
          (:Is%20Not%20Valid
            (Development|PrintString "wompo womp 2"))))
      (:else))))

(event Custom|Kamikaze
  (for _index (range 0 (- (.noofenemies (Variables|Default|GetKamikazeData)) 1))
    (bind _bp_hexgrid (Variables|Default|GetBP_HexGrid)
      (:then
        (bind _tilelocation (Class|IHexGrid|GetRandomTileLocation(Message) _bp_hexgrid))
        (bind _returnvalue (Game|SpawnActorfromClass "/Game/Snowstorm/Systems/Enemies/BP_Enemy02.BP_Enemy02_C" (Math|Transform|MakeTransform (Math|Vector|MakeVector (.x _tilelocation) (.y _tilelocation) (+ (.z _tilelocation) 2e+03)) "0, 0, 0" "2.000000,2.000000,2.000000") "Undefined" "MultiplyWithRoot" 0 0))
        (Utilities|IsValid _returnvalue
          (:Is%20Valid
            (Variables|/Script/Engine.CharacterMovementComponent|SetGravityScale (Variables|/Script/Engine.Character|GetCharacterMovement _returnvalue) (.gravscale (Variables|Default|GetKamikazeData))))
          (:Is%20Not%20Valid
            (Development|PrintString "wompo womp 2"))))
      (:else))))

(event EventBeginPlay)

(event EventTick
  (params (DeltaSeconds :type Float%20%28single-precision%29)))

(event EventToggleEnemySpawning
  (params (EnemyType :type Integer))
  (bind _krakendata (Variables|Default|GetKrakenData))
  (bind _kamikazedata (Variables|Default|GetKamikazeData))
  (bind _zombiedata (Variables|Default|GetZombieData))
  (bind (_mintime _maxtime) (Utilities|Struct|BreakS_EnemyData _zombiedata))
  (bind (_mintime_2 _maxtime_2) (Utilities|Struct|BreakS_EnemyData _krakendata))
  (bind (_mintime_3 _maxtime_3) (Utilities|Struct|BreakS_EnemyData _kamikazedata))
  (switch int EnemyType
    (:0
      (Utilities|FlowControl|FlipFlop
        (:A
          (bind _returnvalue (Utilities|Time|SetTimerbyEvent (EventDispatchers|CreateEvent :!event Custom|Zombies) (Math|Random|RandomFloatinRange _mintime _maxtime) true)))
        (:B
          (Utilities|Time|PauseTimerbyHandle _returnvalue))))
    (:1
      (Utilities|FlowControl|FlipFlop
        (:A
          (bind _returnvalue_2 (Utilities|Time|SetTimerbyEvent (EventDispatchers|CreateEvent :!event Custom|Kamikaze) (Math|Random|RandomFloatinRange _mintime_3 _maxtime_3) true)))
        (:B
          (Utilities|Time|PauseTimerbyHandle _returnvalue_2))))
    (:2
      (Utilities|FlowControl|FlipFlop
        (:A
          (bind _returnvalue_3 (Utilities|Time|SetTimerbyEvent (EventDispatchers|CreateEvent :!event Custom|Kraken) (Math|Random|RandomFloatinRange _mintime_2 _maxtime_2) true)))
        (:B
          (Utilities|Time|PauseTimerbyHandle _returnvalue_3))))))

(fn ConstructionScript)

(fn RegisterHexGridActor
  (params (HexGridRef :type BP%20Hex%20Grid%20Object%20Reference))
  (bind _output_get (Variables|Default|SetBP_HexGrid HexGridRef))
  (return (Utilities|IsValid _output_get)))