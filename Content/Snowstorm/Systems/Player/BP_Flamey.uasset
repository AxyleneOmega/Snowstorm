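; BP_Flamey is the Snowstorm player character, whose toggleable melting powers break tiles underfoot.
; A looping timer traces downward and messages the hit actor with current and previous item indices, while a landing trace activates a Niagara effect.
; Ocean overlap triggers delayed game over and self-destruction, which asks the game mode to reset.
; Debug keys toggle GameMode enemy spawning, and G regenerates the BP_HexGrid tiles.
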(event Custom|FootTrace
  (bind _returnvalue (Transformation|GetActorLocation))
  (bind _outhit (Collision|LineTraceByChannel _returnvalue (+ _returnvalue (* (Math|Vector|NegateVector (Transformation|GetActorUpVector)) 200)) "TraceTypeQuery1" false 0 "None" true "(R=1.000000,G=0.000000,B=0.000000,A=1.000000)" "(R=0.000000,G=1.000000,B=0.000000,A=1.000000)" 2.0))
  (Class|IHexGrid|BreakTileonCollision(Message) (.HitActor (Collision|BreakHitResult _outhit)) (.HitItem (Collision|BreakHitResult _outhit)) (Variables|Default|GetHit%20Item))
  (Variables|Default|SetHit%20Item (.HitItem (Collision|BreakHitResult _outhit))))

(event Custom|CustomEvent
  (bind _returnvalue (Transformation|GetActorLocation))
  (bind _returnvalue_2 (Collision|LineTraceByChannel _returnvalue (+ _returnvalue (* (Math|Vector|NegateVector (Transformation|GetActorUpVector)) 100)) "TraceTypeQuery1" false 0 "None" true "(R=1.000000,G=0.000000,B=0.000000,A=1.000000)" "(R=0.000000,G=1.000000,B=0.000000,A=1.000000)" 2.0))
  (if _returnvalue_2
    (Components|Activation|Activate (Variables|Default|GetNewNiagaraSystem1) true)
    (Utilities|Time|PauseTimerbyHandle (stale Custom|CharacterLanded _returnvalue))))

(event Custom|ToggleMeltingPowers
  (if (Utilities|Time|IsTimerActivebyHandle (Variables|Default|GetFootTraceHandle))
    (Utilities|Time|ClearandInvalidateTimerbyHandle (Variables|Default|GetFootTraceHandle))
    (else
      (bind _returnvalue (Utilities|Time|SetTimerbyEvent (delegate Custom|FootTrace) 0.1 true))
      (Variables|Default|SetFootTraceHandle _returnvalue))))

(event Custom|CharacterLanded
  (bind _returnvalue (Utilities|Time|SetTimerbyEvent (delegate Custom|CustomEvent) 0.1 true)))

(event EventBeginPlay)

(event Collision|EventActorBeginOverlap
  (params (OtherActor :type Actor%20Object%20Reference)))

(event EventOnOverlapOcean
  (Utilities|FlowControl|Delay 1.0)
  (Class|IPC|OnGameOver(Message) (Game|GetPlayerController 0))
  (Actor|DestroyActor))

(event EventDestroyed
  (Class|IGM|ResetGame(Message) (Game|GetGameMode)))

(event EventTick
  (params (DeltaSeconds :type Float%20%28single-precision%29)))

(event Input|KeyboardEvents|DebugKey1
  (params (Key :type Key%20Structure :default "None") (ActionValue :type Input%20Action%20Value%20Structure))
  ;[0.009375 0.009375 0.009375] Enemy Spawner (See GM_SS - GameMode for Spawning Implementation)
  (:Pressed
    (Class|IGM|ToggleEnemySpawning(Message) (Game|GetGameMode) 1)))

(event Input|KeyboardEvents|DebugKey2
  (params (Key :type Key%20Structure :default "None") (ActionValue :type Input%20Action%20Value%20Structure))
  ;[0.009375 0.009375 0.009375] Enemy Spawner (See GM_SS - GameMode for Spawning Implementation)
  (:Pressed
    (Class|IGM|ToggleEnemySpawning(Message) (Game|GetGameMode) 2)))

(event Input|KeyboardEvents|DebugKey3
  (params (Key :type Key%20Structure :default "None") (ActionValue :type Input%20Action%20Value%20Structure))
  ;[0.009375 0.009375 0.009375] Enemy Spawner (See GM_SS - GameMode for Spawning Implementation)
  (:Pressed
    (Class|IGM|ToggleEnemySpawning(Message) (Game|GetGameMode) 3)))

(event Input|KeyboardEvents|G
  (params (Key :type Key%20Structure :default "None"))
  (:Pressed
    (bind _returnvalue (Actor|GetActorOfClass "/Game/Snowstorm/HexGrid/BPHexGridSystem/BP_HexGrid.BP_HexGrid_C"))
    (Class|IHexGrid|RegenerateTiles(Message) _returnvalue true (Utilities|Set|MakeSet 0))))

(fn ConstructionScript
  (Transformation|AttachComponentToComponent (Variables|Default|GetNiagara) (Variables|Character|GetMesh) "Bone_007" "KeepRelative" "KeepWorld" "KeepRelative" true))