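; Tentacle enemy character that halts with a water splash once its capsule is at or above Z zero, or shortly after a hit.
; It runs a looping timer while suspended, then restores strong gravity and destroys itself.
; Capsule hits send a break-tile message to the struck actor.
; FirstLerp uses a timeline to lerp the tentacle AnimBP's effector toward a randomized raised point.
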(event OnComponentHit(CapsuleComponent)
  (params (HitComponent :type Primitive%20Component%20Object%20Reference) (OtherActor :type Actor%20Object%20Reference) (OtherComp :type Primitive%20Component%20Object%20Reference) (NormalImpulse :type Vector :default "0, 0, 0") (Hit :type Hit%20Result%20Structure%20%28by%20ref%29))
  (bind (_bblockinghit _binitialoverlap _time _distance _location _impactpoint _normal _impactnormal _physmat _hitactor _hitcomponent _hitbonename _bonename _hititem) (Collision|BreakHitResult Hit))
  (bind _charactermovement (Variables|Character|GetCharacterMovement))
  (Class|IHexGrid|BreakTileonCollision(Message) _hitactor 0 _hititem)
  (Variables|Default|SetHit true)
  (Utilities|FlowControl|Delay 0.5)
  (Components|Activation|Activate (Variables|Default|GetN_WaterSplash) true)
  (Variables|/Script/Engine.CharacterMovementComponent|SetGravityScale _charactermovement 0.0)
  (Variables|/Script/Engine.MovementComponent|SetVelocity _charactermovement "0, 0, 0")
  (bind _returnvalue (Utilities|Time|SetTimerbyEvent (EventDispatchers|CreateEvent :!event Custom|FirstLerp) 0.1 true))
  (Utilities|FlowControl|Delay 3.0)
  (Utilities|Time|PauseTimerbyHandle _returnvalue)
  (Variables|/Script/Engine.CharacterMovementComponent|SetGravityScale (Variables|Character|GetCharacterMovement) 5.0)
  (Utilities|FlowControl|Delay 1.0)
  (Actor|DestroyActor))

(event Custom|FirstLerp
  (Components|Timeline|SetPlayRate (Variables|Default|GetTimeline) (/ 1.0 (Variables|Default|GetNew%20Time)))
  (Variables|Default|SetNewVar_0 (Math|Random|RandomFloatinRange -3.1e+02 3.1e+02))
  (Variables|Default|SetNewVar_1 (Math|Random|RandomFloatinRange -62.0 62.0))
  (bind _astentacle_sketchfab_v_0_06new_skeleton_anim_blueprint (Utilities|Casting|CastTotentacle_sketchfab_v0_06new_Skeleton_AnimBlueprint (Components|SkeletalMesh|GetAnimInstance (Variables|Character|GetMesh))))
  (bind _newtrack_0 (Timeline|Timeline PlayFromStart)
    (:Update
      (Variables|/Game/Tenti/tentacle_sketchfab_v0_06new_Skeleton_AnimBlueprint.tentacle_sketchfab_v0_06new_Skeleton_AnimBlueprint_C|SetEffector%20Location _astentacle_sketchfab_v_0_06new_skeleton_anim_blueprint (Math|Vector|Lerp(Vector) (Variables|/Game/Tenti/tentacle_sketchfab_v0_06new_Skeleton_AnimBlueprint.tentacle_sketchfab_v0_06new_Skeleton_AnimBlueprint_C|GetEffector%20Location _astentacle_sketchfab_v_0_06new_skeleton_anim_blueprint) (Math|Vector|MakeVector (Variables|Default|GetNewVar_0) (Variables|Default|GetNewVar_1) 976.911987) _newtrack_0)))))

(event Collision|EventActorBeginOverlap
  (params (OtherActor :type Actor%20Object%20Reference)))

(event EventTick
  (params (DeltaSeconds :type Float%20%28single-precision%29))
  (bind _charactermovement (Variables|Character|GetCharacterMovement))
  (if (>= (.z (Transformation|GetWorldLocation (Variables|Collision|GetCapsuleComponent))) 0.0)
    (if (not (Variables|Default|GetHit))
      (Components|Activation|Activate (Variables|Default|GetN_WaterSplash) true)
      (Variables|/Script/Engine.CharacterMovementComponent|SetGravityScale _charactermovement 0.0)
      (Variables|/Script/Engine.MovementComponent|SetVelocity _charactermovement "0, 0, 0")
      (bind _returnvalue (Utilities|Time|SetTimerbyEvent (EventDispatchers|CreateEvent :!event Custom|FirstLerp) 0.1 true))
      (Utilities|FlowControl|Delay 3.0)
      (Utilities|Time|PauseTimerbyHandle _returnvalue)
      (Variables|/Script/Engine.CharacterMovementComponent|SetGravityScale (Variables|Character|GetCharacterMovement) 5.0)
      (Utilities|FlowControl|Delay 1.0)
      (Actor|DestroyActor))))

(fn ConstructionScript)